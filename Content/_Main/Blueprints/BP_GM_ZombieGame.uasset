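; Game mode for a wave-based zombie game that runs the wave loop, kill count and upgrade refresh.
; Each wave clears upgrades, moves the bubble to the player, resets chaos mode and shows the wave UI.
; A looping timer then spawns ten zombies per wave number at random points, and upgrades respawn.
; ZombieKilled counts down remaining zombies, then announces the wave's end and starts the next.
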(event Custom|Start%20Game
  ;[0.15 0.15 0.15 0.5] Start Game
  (CallFunction|WaveStart))

(event Custom|ZombieKilled
  ;[0.15 0.15 0.15 0.5] Zombie Killed
  (Math|Integer|IncrementInt (Variables|Default|GetEnemyKills)
    (:%20%20
      (bind _result (Math|Integer|DecrementInt (Variables|Default|GetZombies%20Left))
        (:%20%20
          (if (== _result 0)
            (Default|ShowWaveover (Variables|Default|GetBP_player) (Variables|Default|GetCurrentWave))
            (Audio|PlaySoundatLocation "/Game/_Main/Sounds/waveover.waveover" (Transformation|GetWorldLocation (Variables|/Script/Engine.Character|GetMesh (Game|GetPlayerCharacter 0))) "0, 0, 0" 1.0 1.0 0.0 0 0 0 0)
            (CallFunction|WaveIncreament)))))))

(event Custom|Wave%20Increament
  ;[0.15 0.15 0.15 0.5] Increament Wave
  (Math|Integer|IncrementInt (Variables|Default|GetCurrentWave)
    (:%20%20
      (CallFunction|WaveStart))))

(event Custom|Wave%20Start
  ;[0.15 0.15 0.15 0.5] Start Next Wave
  (Utilities|FlowControl|Delay 0.1)
  (Default|RemoveUpgreades (Variables|Default|GetspawnUPgrades))
  (bind _asbp_first_person_character (Utilities|Casting|CastToBP_FirstPersonCharacter (Game|GetPlayerCharacter 0)))
  (Variables|Default|SetBP_player _asbp_first_person_character)
  (bind _returnvalue (Actor|GetActorOfClass "/Game/_Main/Weapons/BP_Bubble.BP_Bubble_C"))
  (Transformation|SetActorLocation _returnvalue (Transformation|GetActorLocation (Variables|Default|GetBP_player)) false false)
  (Variables|/Game/_Main/Blueprints/BP_FirstPersonCharacter.BP_FirstPersonCharacter_C|SetisChaosMode? (Variables|Default|GetBP_player) false)
  (Default|ChaosMode (Variables|Default|GetBP_player))
  (Utilities|FlowControl|Delay 5.0)
  (Default|ShowWaveUI (Variables|Default|GetBP_player) (Variables|Default|GetCurrentWave))
  (Utilities|FlowControl|Delay 2.0)
  (CallFunction|SpawnWaves)
  (if (not (Variables|/Game/_Main/Blueprints/BP_FirstPersonCharacter.BP_FirstPersonCharacter_C|GetisChaosMode? (Variables|Default|GetBP_player)))
    (Default|RespawnUpgrades (Variables|Default|GetspawnUPgrades))))

(event Custom|SpawnWaves
  ;[0.15 0.15 0.15 0.5] Spawn Zombies
  (bind _output_get (Variables|Default|SetZombie%20Total (* (Variables|Default|GetCurrentWave) 10)))
  (bind _output_get_2 (Variables|Default|SetZombies%20Left _output_get))
  (Variables|Default|SetSpawnsLeft _output_get_2)
  (Utilities|Time|SetTimerbyEvent (delegate Custom|SpawnZombies) (Variables|Default|GetSpawnTime) true))

(event Custom|SpawnZombies
  ;[0.15 0.15 0.15 0.5] Spawn Zombies
  (if (> (Variables|Default|GetSpawnsLeft) 0)
    (bind _output_get (Variables|Default|SetspawnLocation (Math|Transform|MakeTransform (Math|Vector|MakeVector (Math|Random|RandomFloatinRange -3.5e+03 3.5e+03) (Math|Random|RandomFloatinRange -3.5e+03 3.5e+03) 125.0) "0, 0, 0" "1.000000,1.000000,1.000000")))
    (Math|Integer|DecrementInt (Variables|Default|GetSpawnsLeft)
      (:%20%20
        (Game|SpawnActorfromClass "/Game/_Main/Zombie/BP_Zombie.BP_Zombie_C" (Math|Transform|MakeTransform (.location _output_get) "0, 0, 0" "1.000000,1.000000,1.000000") "Undefined" "MultiplyWithRoot" 0 0)))))

(event EventBeginPlay
  ;[0.15 0.15 0.15 0.5] Start Game
  (CallFunction|StartGame)
  (bind _returnvalue (Actor|GetActorOfClass "/Game/_Main/Blueprints/BP_SpawnUpgrades.BP_SpawnUpgrades_C"))
  (Variables|Default|SetspawnUPgrades _returnvalue))

(fn ConstructionScript)