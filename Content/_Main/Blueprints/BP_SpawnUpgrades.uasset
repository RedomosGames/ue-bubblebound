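; BP_SpawnUpgrades manages the placement of three upgrade actors in the level, hiding and respawning them.
; Removeupgreades moves all three to one fixed point far away, taking them out of play without destroying them.
; RespawnUpgrades teleports each back to its own random X/Y position within a square area around the world origin at a fixed height, reusing the existing actors instead of spawning new ones.
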(event Custom|RespawnUpgrades
  ;[0.15 0.15 0.15 0.5] Spawn in Upgrade Actors
  (bind _output_get (Variables|Default|SetspawnLocation (Math|Transform|MakeTransform (Math|Vector|MakeVector (Math|Random|RandomFloatinRange -3.5e+03 3.5e+03) (Math|Random|RandomFloatinRange -3.5e+03 3.5e+03) 1.5e+02) "0, 0, 0" "1.000000,1.000000,1.000000")))
  (Transformation|SetActorLocation (Variables|Default|Getupgrade1) (.location _output_get) false false)
  (bind _output_get_2 (Variables|Default|SetspawnLocation (Math|Transform|MakeTransform (Math|Vector|MakeVector (Math|Random|RandomFloatinRange -3.5e+03 3.5e+03) (Math|Random|RandomFloatinRange -3.5e+03 3.5e+03) 1.5e+02) "0, 0, 0" "1.000000,1.000000,1.000000")))
  (Transformation|SetActorLocation (Variables|Default|Getupgrade2) (.location _output_get_2) false false)
  (bind _output_get_3 (Variables|Default|SetspawnLocation (Math|Transform|MakeTransform (Math|Vector|MakeVector (Math|Random|RandomFloatinRange -3.5e+03 3.5e+03) (Math|Random|RandomFloatinRange -3.5e+03 3.5e+03) 1.5e+02) "0, 0, 0" "1.000000,1.000000,1.000000")))
  (Transformation|SetActorLocation (Variables|Default|Getupgrade3) (.location _output_get_3) false false))

(event Custom|Remove%20upgreades
  ;[0.15 0.15 0.15 0.5] Remove Upgrade Actors
  (Transformation|SetActorLocation (Variables|Default|Getupgrade1) "0.000000,10000.000000,10000.000000" false false)
  (Transformation|SetActorLocation (Variables|Default|Getupgrade2) "0.000000,10000.000000,10000.000000" false false)
  (Transformation|SetActorLocation (Variables|Default|Getupgrade3) "0.000000,10000.000000,10000.000000" false false))

(fn ConstructionScript)