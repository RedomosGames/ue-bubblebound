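; BP_Zombie is an enemy character that chases the player and attacks in melee.
; AIMoveTo and a montage attack loop into each other, with damage dealt by a sphere overlap on the montage notify.
; Point damage reduces health and plays hit reactions until death, which notifies BP_GM_ZombieGame and destroys the actor.
; A delayed Tick polls the player's chaos mode to set speed, attack rate and damage, overriding the speed set on sight.
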(event OnSeePawn(PawnSensing)
  (params (Pawn :type Pawn%20Object%20Reference))
  ;[0.15 0.15 0.15 0.5] Run to Player
  (Variables|/Script/Engine.CharacterMovementComponent|SetMaxWalkSpeed (Variables|Character|GetCharacterMovement) 3.6e+02))

(event Custom|RunToPlayer
  ;[0.15 0.15 0.15 0.5] Chase Player
  (if (not (Variables|Default|GetisDead?))
    (AI|AIMoveTo self "0, 0, 0" (Game|GetPlayerController 0) 1.5e+02 false
      (:OnSuccess
        (CallFunction|AttackPlayer))
      (:OnFail
        (CallFunction|RuntoPlayer)))))

(event Custom|AttackPlayer
  ;[0.15 0.15 0.15 0.5] Attack Player
  (Animation|Montage|PlayMontage (Variables|Character|GetMesh) "/Game/_Main/Zombie/Animations/zombie_attack_Montage.zombie_attack_Montage" (Variables|Default|GetAttackSpeed)
    (:OnCompleted
      (CallFunction|RuntoPlayer :!label _label))
    (:OnInterrupted
      (goto _label))
    (:OnNotifyBegin
      (bind (_outactors _returnvalue) (Collision|SphereOverlapActors (Transformation|GetWorldLocation (Variables|Default|GetArrow1)) 1.2e+02 (Utilities|Array|MakeArray "ObjectTypeQuery3") "/Game/_Main/Blueprints/BP_FirstPersonCharacter.BP_FirstPersonCharacter_C" (Utilities|Array|MakeArray self)))
      (if _returnvalue
        (for _array_element _outactors
          (Game|Damage|ApplyDamage _array_element (Variables|Default|GetAttack%20DMG) (Pawn|GetController) self "/Script/Engine.DamageType"))))))

(event Custom|Death
  ;[0.15 0.15 0.15 0.5] Death
  (Variables|Default|SetisDead? true)
  (Components|Movement|StopMovementImmediately (Variables|Character|GetCharacterMovement))
  (Audio|PlaySoundatLocation "/Game/_Main/Sounds/death.death" (Transformation|GetWorldLocation (Variables|/Script/Engine.Character|GetMesh (Game|GetPlayerCharacter 0))) "0, 0, 0" 0.6 1.0 0.0 0 0 0 0)
  (Animation|Montage|PlayMontage (Variables|Character|GetMesh) "/Game/_Main/Zombie/Animations/zombie_dying_Montage.zombie_dying_Montage" 1.2
    (:then
      (Collision|SetCollisionResponsetoChannel (Variables|Collision|GetCapsuleComponent) "ECC_Pawn" "ECR_Overlap")
      (Collision|SetCollisionEnabled (Variables|Character|GetMesh) "NoCollision")
      (bind _asbp_gm_zombie_game (Utilities|Casting|CastToBP_GM_ZombieGame (Game|GetGameMode)))
      (Default|ZombieKilled _asbp_gm_zombie_game)
      (Utilities|FlowControl|Delay 3.0)
      (Actor|DestroyActor))))

(event Custom|ChaosMode
  (bind _charactermovement (Variables|Character|GetCharacterMovement))
  ;[0.15 0.15 0.15 0.5] Choas MOde
  (if (Variables|/Game/_Main/Blueprints/BP_FirstPersonCharacter.BP_FirstPersonCharacter_C|GetisChaosMode? (Variables|Default|Getbp_Player))
    (Variables|/Script/Engine.CharacterMovementComponent|SetMaxWalkSpeed _charactermovement 1.1e+03)
    (Variables|Default|SetAttackSpeed 2.0)
    (Variables|Default|SetAttack%20DMG 4e+01)
    (else
      (Variables|/Script/Engine.CharacterMovementComponent|SetMaxWalkSpeed _charactermovement 5e+02)
      (Variables|Default|SetAttackSpeed 1.0)
      (Variables|Default|SetAttack%20DMG 2e+01))))

(event EventBeginPlay
  ;[0.15 0.15 0.15 0.5] Begin Play
  (Utilities|FlowControl|Delay 1.0)
  (CallFunction|RuntoPlayer)
  (bind _asbp_first_person_character (Utilities|Casting|CastToBP_FirstPersonCharacter (Game|GetPlayerCharacter 0)))
  (Variables|Default|Setbp_Player _asbp_first_person_character))

(event Game|Damage|EventPointDamage
  (params (Damage :type Float%20%28single-precision%29) (DamageType :type Damage%20Type%20Object%20Reference) (HitLocation :type Vector :default "0, 0, 0") (HitNormal :type Vector :default "0, 0, 0") (HitComponent :type Primitive%20Component%20Object%20Reference) (BoneName :type Name :default "None") (ShotFromDirection :type Vector :default "0, 0, 0") (InstigatedBy :type Controller%20Object%20Reference) (DamageCauser :type Actor%20Object%20Reference) (HitInfo :type Hit%20Result%20Structure%20%28by%20ref%29))
  ;[0.15 0.15 0.15 0.5] Take DMG
  (if (not (Variables|Default|GetisDead?))
    (if (<= (Variables|Default|GetHealth) 0.0)
      (CallFunction|Death)
      (else
        (bind _output_get (Variables|Default|SetHealth (- (Variables|Default|GetHealth) Damage)))
        (Development|PrintString (Utilities|String|ToString(Float) _output_get))
        (if (<= (Variables|Default|GetHealth) 0.0)
          (CallFunction|Death)
          (else
            (Animation|Montage|PlayMontage (Variables|Character|GetMesh) "/Game/_Main/Zombie/Animations/Zombie_Reaction_Hit_Montage.Zombie_Reaction_Hit_Montage")))))))

(event EventTick
  (params (DeltaSeconds :type Float%20%28single-precision%29))
  ;[0.15 0.15 0.15 0.5] Choas MOde
  (Utilities|FlowControl|Delay 0.1)
  (CallFunction|ChaosMode))

(fn ConstructionScript)